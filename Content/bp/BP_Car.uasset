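; BP_Car is a car Blueprint that, as shown, only registers its four suspension top links and four wheels.
; On BeginPlay, a loop uses Select by index to fill the Links and Wheels arrays in matching front-left, front-right, rear-left, rear-right order.
; Tick, overlap and the construction script are empty, so no driving or suspension logic runs in these graphs.
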(event EventBeginPlay
  (for _index (range 0 3)
    (Utilities|Array|AddUnique (Variables|Default|GetLinks) (Utilities|Select :Index _index :Option%200 (Variables|Default|GetTopLink_FL) :Option%201 (Variables|Default|GetTopLink_FR) :Option%202 (Variables|Default|GetTopLink_RL) :Option%203 (Variables|Default|GetTopLink_RR)))
    (Utilities|Array|AddUnique (Variables|Default|GetWheels) (Utilities|Select :Index _index :Option%200 (Variables|Default|GetWheel_FL) :Option%201 (Variables|Default|GetWheel_FR) :Option%202 (Variables|Default|GetWheel_RL) :Option%203 (Variables|Default|GetWheel_RR)))))

(event Collision|EventActorBeginOverlap
  (params (OtherActor :type Actor%20Object%20Reference)))

(event EventTick
  (params (DeltaSeconds :type Float%20%28single-precision%29)))

(fn ConstructionScript)